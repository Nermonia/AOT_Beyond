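; Effect actor for the human spinning attack, with an animated skeletal mesh plus blood and smoke trail components.
; On BeginPlay the mesh plays its spinning attack rig montage once.
; Tick forces both particle components to unit world scale so they ignore inherited scaling.
; Kill hides only the mesh, not its children, then destroys the actor after a short delay.
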(event `self.ReceiveBeginPlay`
  (`SkeletalMeshComponent.PlayAnimation` (`self.SkeletalMesh`) "/Game/Art/Effect/Combat/Spinning_Attack/Anims/Effect_SpinningAttack_01_RIG_Montage.Effect_SpinningAttack_01_RIG_Montage" false))

(event `Kill`
  (`SceneComponent.SetHiddenInGame` (`self.SkeletalMesh`) true false)
  (`KismetSystemLibrary.Delay` 2.0)
  (`self.K2_DestroyActor`))

(event `self.ReceiveTick`
  (params (DeltaSeconds :type "Float (single-precision)"))
  (`SceneComponent.SetWorldScale3D` (`self.Blood Particle`) (1.0 1.0 1.0))
  (`SceneComponent.SetWorldScale3D` (`self.Smoke Trail`) (1.0 1.0 1.0)))

(fn `UserConstructionScript`)