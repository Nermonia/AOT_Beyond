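; Titan enemy character that spots, grabs, eats and attacks the player, and dies when struck at the nape.
; Tick runs death, sight and animation updates, using gated overlap volumes, line traces and smoothed rotation.
; Attack events drive the AnimBP; sphere-traced catches report to the Blackboard or trigger dodge counters for invincible players.
; Counter feedback uses a dynamic skin material, arm ragdoll and blood splats; death triggers an explosion and full ragdoll.
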(event `self.ReceiveBeginPlay`
  ;[1 1 1] Begin
  (bind _returnvalue (`AIBlueprintHelperLibrary.GetAIController` self))
  (bind _output_get (set `self.Blackboard` (`AIBlueprintHelperLibrary.GetBlackboard` _returnvalue)))
  (`/Engine/EditorBlueprintResources/StandardMacros.IsValid` _output_get
    (:`Is Valid`
      (`BlackboardComponent.SetValueAsBool` (`self.Blackboard`) "CanAttack?" true) ; As soon as he spawns, the player can attack
      (bind _asanim_bp_big_titan_01 (cast `/Game/Animations/Titan/BigTitan/AnimBP_Big_Titan01` (`SkeletalMeshComponent.GetAnimInstance` (`self.Mesh`))))
      (set `self.AnimBP` _asanim_bp_big_titan_01)
      (bind _returnvalue_2 (`PrimitiveComponent.CreateDynamicMaterialInstance` (`self.Mesh`) 1 "/Game/Art/Character/Titan/Shaders/INST_BigTitan01_Body.INST_BigTitan01_Body"))
      (set `self.Titan Skin Shader` _returnvalue_2))))

(event `self.NeckDamageVolume.OnComponentBeginOverlap`
  (params (OverlappedComponent :type "PrimitiveComponent Object Reference") (OtherActor :type "Actor Object Reference") (OtherComp :type "PrimitiveComponent Object Reference") (OtherBodyIndex :type Integer) (bFromSweep :type Boolean) (SweepResult :type "HitResult Structure (by ref)"))
  (bind _mesh (`self.Mesh`))
  (bind _player (`self.Player`))
  (bind (_returnvalue_x _returnvalue_y _returnvalue_z) (`KismetMathLibrary.BreakVector` (`SceneComponent.GetSocketLocation` _mesh "head")))
  ;[1 1 1] Tick
  (goto _label_2 :!via `Open`))

(event `self.NeckDamageVolume.OnComponentEndOverlap`
  (params (OverlappedComponent :type "PrimitiveComponent Object Reference") (OtherActor :type "Actor Object Reference") (OtherComp :type "PrimitiveComponent Object Reference") (OtherBodyIndex :type Integer))
  (bind _mesh (`self.Mesh`))
  (bind _player (`self.Player`))
  (bind (_returnvalue_x _returnvalue_y _returnvalue_z) (`KismetMathLibrary.BreakVector` (`SceneComponent.GetSocketLocation` _mesh "head")))
  ;[1 1 1] Tick
  (bind _asbp_main_character (cast `/Game/Art/Character/MainCharacter/BP_MainCharacter` OtherActor))
  (clear `/Game/Art/Character/MainCharacter/BP_MainCharacter.AttackKey Released` _asbp_main_character)
  (goto _label_2 :!via `Close`))

(event `Attack`
  (bind _mesh (`self.Mesh`))
  (bind _player (`self.Player`))
  (bind (_returnvalue_x _returnvalue_y _returnvalue_z) (`KismetMathLibrary.BreakVector` (`SceneComponent.GetSocketLocation` _mesh "head")))
  ;[1 1 1] Tick
  (`/Engine/EditorBlueprintResources/StandardMacros.Gate` true :!label _label
    (:`Exit`
      (set `self.IsDead?` true)
      (`/Game/Art/Character/MainCharacter/BP_MainCharacter.StopUpdateLeftCable` _player)
      (`/Game/Art/Character/MainCharacter/BP_MainCharacter.StopUpdateRightCable` _player)
      (`PrimitiveComponent.SetCollisionEnabled` (`self.CapsuleComponent`) "NoCollision")
      (`PrimitiveComponent.SetCollisionResponseToChannel` _mesh "ECC_Pawn" "ECR_Ignore") ; Deactivate collision with player
      (bind _returnvalue (`GameplayStatics.SpawnEmitterAtLocation` "/Game/Art/Effect/Particles/P_Explosion.P_Explosion" (`KismetMathLibrary.MakeVector` _returnvalue_x (- _returnvalue_y 200.0) _returnvalue_z)))
      (`SceneComponent.SetWorldScale3D` _returnvalue (10.0 10.0 10.0)) ; Spawn Effect and scale it
      (`SceneComponent.K2_AddLocalRotation` (`self.Mesh`) (struct :`Roll` -10.0) false false)
      (`KismetSystemLibrary.Delay` 0.1)
      (`PrimitiveComponent.SetSimulatePhysics` (`self.Mesh`) true) ; After a delay, activate the ragdoll
      (`KismetSystemLibrary.Delay` 10.0)
      (`self.K2_DestroyActor`) ; After a delay, destroy the titan
    )))

(event `self.ReceiveTick`
  (params (DeltaSeconds :type "Float (single-precision)"))
  (bind _blackboard (`self.Blackboard`))
  ;[1 1 1] Tick
  (set `self.Delta` DeltaSeconds)
  (`|ExecutionSequence`
    (:`then_0`
      (`/Engine/EditorBlueprintResources/StandardMacros.Gate` true :!label _label_2
        (:`Exit`
          (bind _asbp_main_character (cast `/Game/Art/Character/MainCharacter/BP_MainCharacter` (stale `self.NeckDamageVolume.OnComponentBeginOverlap` OtherActor)))
          (set `self.Player` _asbp_main_character)
          (bind _result (`self.TestDistance` (`SceneComponent.GetSocketLocation` (`self.Mesh`) "Nape") (`self.K2_GetActorLocation` (`self.Player`)) 500.0))
          (if _result
            (add `/Game/Art/Character/MainCharacter/BP_MainCharacter.AttackKey Released` (`self.Player`) (delegate `Attack`))
            (goto _label :!via `Open`)))))
    (:`then_1`
      (`/Engine/EditorBlueprintResources/StandardMacros.Gate` true :!label _label_3
        (:`Exit`
          (bind _output_get (set `self.TargetLocation` (`self.K2_GetActorLocation` (`self.Target`))))
          (bind (_outhit _returnvalue) (`KismetSystemLibrary.LineTraceSingle` (`SceneComponent.GetSocketLocation` (`self.Mesh`) "head") _output_get "TraceTypeQuery1"))
          (if _returnvalue
            (set `self.SeePlayer?` false)
            (else
              (set `self.SeePlayer?` true)
              (`self.SeePlayer` (`self.Target`)))))))
    (:`then_2`
      (`self.K2_SetActorRotation` (`KismetMathLibrary.RInterpTo` (`self.K2_GetActorRotation`) (`self.DesiredRotation`) (`GameplayStatics.GetWorldDeltaSeconds`) 7.0)) ; I use an RInterp node so the character smoothly reach the desired rotation instead of poping
      (`/Engine/EditorBlueprintResources/StandardMacros.IsValid` _blackboard
        (:`Is Valid`
          (bind _asbp_main_character_2 (cast `/Game/Art/Character/MainCharacter/BP_MainCharacter` (`BlackboardComponent.GetValueAsObject` _blackboard "TargetActor")))
          (`SceneComponent.K2_SetWorldRotation` (`self.HeadLookAtAngleInvestigator`) (`KismetMathLibrary.FindLookAtRotation` (`SceneComponent.K2_GetComponentLocation` (`self.HeadLookAtAngleInvestigator`)) (`self.K2_GetActorLocation` _asbp_main_character_2)) false false) ; The "head look at Investigator" \nmust always face the target, as \nit'll be used in the BP Anim to rotate the head of the Titan
        )))))

(event `self.VisionCone.OnComponentBeginOverlap`
  (params (OverlappedComponent :type "PrimitiveComponent Object Reference") (OtherActor :type "Actor Object Reference") (OtherComp :type "PrimitiveComponent Object Reference") (OtherBodyIndex :type Integer) (bFromSweep :type Boolean) (SweepResult :type "HitResult Structure (by ref)"))
  ;[1 1 1] Tick
  (bind _asbp_main_character (cast `/Game/Art/Character/MainCharacter/BP_MainCharacter` OtherActor))
  (set `self.Target` _asbp_main_character)
  (goto _label_3 :!via `Open`))

(event `self.VisionCone.OnComponentEndOverlap`
  (params (OverlappedComponent :type "PrimitiveComponent Object Reference") (OtherActor :type "Actor Object Reference") (OtherComp :type "PrimitiveComponent Object Reference") (OtherBodyIndex :type Integer))
  ;[1 1 1] Tick
  (cast `/Game/Art/Character/MainCharacter/BP_MainCharacter` OtherActor)
  (set `self.SeePlayer?` false)
  (goto _label_3 :!via `Close`))

(event `ResetPlayerDodged`
  ;[1 1 1] Try to Catch
  (goto _label_4 :!via `Reset`))

(event `Try to Catch`
  (bind _returnvalue (`SceneComponent.GetSocketLocation` (`self.Mesh`) (`self.CatchPlayerLocation`)))
  ;[1 1 1] Try to Catch
  (if (`self.Counter Left/Right`)
    (set `self.CatchPlayerLocation` "hand_l_CatchPlayerLocation")
    (else
      (set `self.CatchPlayerLocation` "hand_r_CatchPlayerLocation")))
  (bind (_outhit _returnvalue_2) (`KismetSystemLibrary.SphereTraceSingleForObjects` _returnvalue (+ _returnvalue 100.0) (`self.CatchAttack01Radius`) (`|MakeArray` "ObjectTypeQuery3" :!type "EObjectTypeQuery Enum"))) ; We do a sphere trace and check if we caught any Pawn
  (if _returnvalue_2
    (bind _asbp_main_character (cast `/Game/Art/Character/MainCharacter/BP_MainCharacter` (`.HitActor` (`GameplayStatics.BreakHitResult` _outhit))))
    (bind _output_get (set `self.TargetPlayer` _asbp_main_character))
    (if (`/Game/Art/Character/MainCharacter/BP_MainCharacter.IsInvincible` _output_get)
      (`/Engine/EditorBlueprintResources/StandardMacros.DoOnce` false :!label _label_4
        (:`Completed`
          (`self.PlayerDodged`)
          (`/Game/Art/Character/MainCharacter/BP_MainCharacter.Listen Counter Input` (`self.TargetPlayer`) (`self.Counter Left/Right`) self (`/Game/Animations/Titan/BigTitan/AnimBP_Big_Titan01.AttackType` (`self.AnimBP`)))))
      (elif (< (`KismetMathLibrary.VSize` (- (`SceneComponent.GetSocketLocation` (`self.Mesh`) (`self.CatchPlayerLocation`)) (`self.K2_GetActorLocation` (`self.Target`)))) (/ (`self.CatchAttack01Radius`) 1.5))
        (cast `SkeletalMeshComponent` (`.HitComponent` (`GameplayStatics.BreakHitResult` _outhit)))
        (`/Game/Art/Character/MainCharacter/BP_MainCharacter.Caught` (`self.TargetPlayer`) self (`self.CatchPlayerLocation`)) ; If we caught a Player, we trigger his Caught event
        (`BlackboardComponent.SetValueAsBool` (`self.Blackboard`) "CaughtPlayer?" true) ; We tell the Behavior Tree that we caught someting so we can launch the Eat animation
      ))))

(event `Try to Eat`
  (bind _blackboard (`self.Blackboard`))
  ;[1 1 1] Try to Eat
  (`/Engine/EditorBlueprintResources/StandardMacros.IsValid` _blackboard
    (:`Is Valid`
      (bind _asbp_main_character (cast `/Game/Art/Character/MainCharacter/BP_MainCharacter` (`BlackboardComponent.GetValueAsObject` _blackboard "TargetActor")))
      (if (< (`KismetMathLibrary.VSize` (- (`self.K2_GetActorLocation` _asbp_main_character) (`SceneComponent.GetSocketLocation` (`self.Mesh`) "Mounth"))) (`self.BiteAttack01Radius`))
        (`/Game/Art/Character/MainCharacter/BP_MainCharacter.Killed` _asbp_main_character)))))

(event `PlayerDodged`
  ;[1 1 1] Player Dodge
  (`BlackboardComponent.SetValueAsBool` (`self.Blackboard`) "TargetDodged" true)
  (`/Game/Animations/Titan/BigTitan/AnimBP_Big_Titan01.PlayerDodged` (`self.AnimBP`)))

(event `PlayerDodgedEnd`
  ;[1 1 1] Player Dodge
  (`/Game/Animations/Titan/BigTitan/AnimBP_Big_Titan01.PlayerDodgeEnd` (`self.AnimBP`))
  (`BlackboardComponent.SetValueAsBool` (`self.Blackboard`) "TargetDodged" false))

(event `Arm Blood Splat`
  (bind _returnvalue (`|SpawnActorFromClass` "/Game/Temp/BloodSplat_Arm/BP_BloodSplat_Arm01.BP_BloodSplat_Arm01_C" (`KismetMathLibrary.MakeTransform` (0.0 0.0 0.0) (struct) (12.0 12.0 12.0)) "AlwaysSpawn" "OverrideRootScale"))
  (if (`/Game/Art/Character/MainCharacter/BP_MainCharacter.Counter_Left/Right` (`self.TargetPlayer`))
    (`self.K2_AttachRootComponentTo` _returnvalue (`self.Mesh`) "upperarm_l" "SnapToTarget" false)
    (else
      (`self.K2_AttachRootComponentTo` _returnvalue (`self.Mesh`) "upperarm_r" "SnapToTarget" false))))

(event `/Game/Art/Character/Titan/BPI_Titan_PlayAnim.Titan_Attack`
  (params (AttackType :type Byte :default 0) (PlayRate :type "Float (single-precision)") (DelayBetweenAttacks :type "Float (single-precision)") (OverrideDelayBetweenAttack :type Boolean))
  (set `self.Attack Type` AttackType)
  (if (not OverrideDelayBetweenAttack)
    (set `self.Delay Between Attack` DelayBetweenAttacks)
    (`/Engine/EditorBlueprintResources/StandardMacros.DoOnce` false :!label _label_5
      (:`Completed`
        (switch `|SwitchEnum` (`self.Attack Type`)
          (:`NewEnumerator0`
            (`/Game/Animations/Titan/BigTitan/AnimBP_Big_Titan01.Mounth Attack` (`self.AnimBP`)))
          (:`NewEnumerator3`
            (set `self.Counter Left/Right` true)
            (`/Game/Animations/Titan/BigTitan/AnimBP_Big_Titan01.Catch Attack` (`self.AnimBP`) (`self.Counter Left/Right`) :!label _label_6))
          (:`NewEnumerator5`
            (set `self.Counter Left/Right` false)
            (goto _label_6))
          (:`NewEnumerator4`
            (`/Game/Animations/Titan/BigTitan/AnimBP_Big_Titan01.Eat Attack` (`self.AnimBP`)))
          (:`NewEnumerator6`
            (set `self.Counter Left/Right` true)
            (`/Game/Animations/Titan/BigTitan/AnimBP_Big_Titan01.Stomp Attack` (`self.AnimBP`) (`self.Counter Left/Right`))))
        (`/Game/Animations/Titan/BigTitan/AnimBP_Big_Titan01.Listen to Player Location` (`self.AnimBP`))
        (`KismetSystemLibrary.Delay` (`self.Delay Between Attack`))
        (`self.Reset Attack Timer`)))))

(event `Reset Attack Timer`
  (goto _label_5 :!via `Reset`))

(event `Arm Ragdoll`
  (if (`self.Counter Left/Right`)
    (`SkeletalMeshComponent.SetAllBodiesBelowSimulatePhysics` (`self.Mesh`) "upperarm_l" true true)
    (else
      (`SkeletalMeshComponent.SetAllBodiesBelowSimulatePhysics` (`self.Mesh`) "upperarm_r" true true))))

(event `Apply Counter Effect`
  (params (Boolean :type Boolean))
  (if Boolean
    (`MaterialInstanceDynamic.SetScalarParameterValue` (`self.Titan Skin Shader`) "Counter Intensity" 1.0)
    (else
      (`MaterialInstanceDynamic.SetScalarParameterValue` (`self.Titan Skin Shader`) "Counter Intensity" 0.0))))

(fn `TestDistance`
  (params (HomeLocation :type "Vector Structure" :default (0.0 0.0 0.0)) (TargetLocation :type "Vector Structure" :default (0.0 0.0 0.0)) (DistanceToTest :type "Float (double-precision)" :default 0.0))
  (returns (Result :type Boolean))
  (return (< (`KismetMathLibrary.VSize` (- HomeLocation TargetLocation)) DistanceToTest)))

(fn `UserConstructionScript`
  (bind _neckdamagevolume (`self.NeckDamageVolume`))
  (`|ExecutionSequence`
    (:`then_0`
      (`SceneComponent.K2_AttachTo` _neckdamagevolume (`self.Mesh`) "neck_01" "SnapToTarget" true) ; When the player is inside this volume, I'm listening if he press \nthe Attack input to call the death of the Titan
      (`SceneComponent.K2_AddLocalOffset` _neckdamagevolume (0.0 -150.0 0.0) false false)
      (`SceneComponent.K2_AttachTo` (`self.VisionCone`) (`self.Mesh`) "head" "KeepRelativeOffset" false) ; I attach the vision cone to the head
    )))