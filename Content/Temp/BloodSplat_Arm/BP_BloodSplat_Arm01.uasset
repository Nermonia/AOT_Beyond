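; BP_BloodSplat_Arm01 is a short-lived blood splat effect actor that animates its BloodArmSplat01 component, then destroys itself.
; Tick plays the Particle_Time timeline, whose SizeScale track drives time, opacity fade, dissolve and flow-map intensity in the SmokeVFX Material Parameter Collection and grows the component in X and Z.
; Those parameters live in the shared collection, so they are global; the material cached on BeginPlay goes unused.
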(event `self.ReceiveBeginPlay`
  (set `self.Material` (`PrimitiveComponent.GetMaterial` (`self.BloodArm_Splat01`) 0)))

(event `self.ReceiveTick`
  (params (DeltaSeconds :type "Float (single-precision)"))
  (bind _sizescale (`self.SizeScale`))
  (bind _returnvalue (+ (* _sizescale (`self.SizeOverLifeMultiplier`)) 1.0))
  (bind (_direction _sizescale_2) (`Timeline|Particle_Time`)
    (:`Update`
      (set `self.SizeScale` _sizescale_2)
      (`KismetMaterialLibrary.SetScalarParameterValue` "/Game/Temp/SmokeVFX.SmokeVFX" "Time" (`self.SizeScale`))
      (`KismetMaterialLibrary.SetScalarParameterValue` "/Game/Temp/SmokeVFX.SmokeVFX" "ParticleOpacity" (`KismetMathLibrary.FClamp` (* (- 1.0 (`self.SizeScale`)) 2.0)))
      (`KismetMaterialLibrary.SetScalarParameterValue` "/Game/Temp/SmokeVFX.SmokeVFX" "AlphaDissolve" _sizescale)
      (`KismetMaterialLibrary.SetScalarParameterValue` "/Game/Temp/SmokeVFX.SmokeVFX" "FlowMapIntensity" _sizescale)
      (`SceneComponent.SetRelativeScale3D` (`self.BloodArm_Splat01`) (`KismetMathLibrary.MakeVector` _returnvalue 1.0 _returnvalue)))
    (:`Finished`
      (`self.K2_DestroyActor`))))

(fn `UserConstructionScript`)