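; BP_AttackSlash is a short-lived attack slash effect that fades its visuals and then removes itself.
; BeginPlay creates dynamic material instances for the SmallSlash and LongSlash components.
; Tick interpolates one shared Opacity toward zero, once per material so twice each frame, feeding each instance's "Opacity Multiplier" parameter.
; A Delay on the same Tick sequence destroys the actor after a few seconds.
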(event `self.ReceiveBeginPlay`
  (bind _longslash (`self.LongSlash`))
  (bind _smallslash (`self.SmallSlash`))
  ;[1 1 1] Initialize
  (bind _returnvalue (`PrimitiveComponent.CreateDynamicMaterialInstance` _smallslash 0 (`PrimitiveComponent.GetMaterial` _smallslash 0)))
  (set `self.Material 01` _returnvalue)
  (bind _returnvalue_2 (`PrimitiveComponent.CreateDynamicMaterialInstance` _longslash 0 (`PrimitiveComponent.GetMaterial` _longslash 0)))
  (set `self.Material 02` _returnvalue_2))

(event `self.ReceiveTick`
  (params (DeltaSeconds :type "Float (single-precision)"))
  (`|ExecutionSequence`
    (:`then_0`
      (set `self.Opacity` (`KismetMathLibrary.FInterpTo` (`self.Opacity`) 0.0 (`GameplayStatics.GetWorldDeltaSeconds`) 5.0))
      (`MaterialInstanceDynamic.SetScalarParameterValue` (`self.Material 01`) "Opacity Multiplier" (`self.Opacity`)))
    (:`then_1`
      (set `self.Opacity` (`KismetMathLibrary.FInterpTo` (`self.Opacity`) 0.0 (`GameplayStatics.GetWorldDeltaSeconds`) 5.0))
      (`MaterialInstanceDynamic.SetScalarParameterValue` (`self.Material 02`) "Opacity Multiplier" (`self.Opacity`)))
    (:`then_2`
      (`KismetSystemLibrary.Delay` 3.0)
      (`self.K2_DestroyActor`))))

(fn `UserConstructionScript`)