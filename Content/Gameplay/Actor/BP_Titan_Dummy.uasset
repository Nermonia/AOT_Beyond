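; Titan training dummy that optionally rotates on a timeline, from a set or random orientation, and has a neck the player can cut once.
; Capsule overlap registers the attack-release callback with the player and opens a gate, which closes on exit.
; A cut notifies score and movement, spawns slash and sparks, and swaps the neck for a launched physics piece.
; Pawn collision and camera collision testing switch off briefly so the player passes through.
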(event `self.ReceiveBeginPlay`
  (if (`self.StartRotating?`)
    (if (`self.RandomInitialOrientation?`)
      (bind _output_get (set `self.InitialOrientation` (`KismetMathLibrary.RandomFloatInRange` 0.0 (`TimelineComponent.GetTimelineLength` (`self.Rotation`))))))
    (`TimelineComponent.SetNewTime` (`self.Rotation`) _output_get)
    ;[1 1 1] Comment
    (`self.Start Rotating`)
    (`PrimitiveComponent.SetCollisionEnabled` (`self.NeckCut`) "QueryOnly")))

(event `Start Rotating`
  (bind (_direction _rotation) (`Timeline|Rotation` :!label _label)
    (:`Update`
      (`SceneComponent.K2_SetRelativeRotation` (`self.Dummy`) (`KismetMathLibrary.MakeRotator` 0.0 0.0 _rotation) false false))))

(event `Stop Rotating`
  (goto _label :!via `Stop`))

(event `AttackKey Released`
  (if (not (`self.HasBeenCut?`))
    (`/Engine/EditorBlueprintResources/StandardMacros.Gate` true :!label _label_2
      (:`Exit`
        (`|ExecutionSequence`
          (:`then_0`
            (`self.Set Player Invincible` 0.5))
          (:`then_1`
            (set `self.HasBeenCut?` true)
            (`self.Display Attack Slash`)
            (`/Game/Gameplay/Training/Score.Apply Attack Intensity Score` (`/Game/Art/Character/MainCharacter/BP_MainCharacter.Score` (`self.PlayerAttack`)))
            (message `/Game/Gameplay/Movement/BPI_PlayerInteraction.HitTitan` (`/Game/Art/Character/MainCharacter/BP_MainCharacter.PlayerMovement` (`self.PlayerAttack`)))))))))

(event `self.Capsule.OnComponentBeginOverlap`
  (params (OverlappedComponent :type "PrimitiveComponent Object Reference") (OtherActor :type "Actor Object Reference") (OtherComp :type "PrimitiveComponent Object Reference") (OtherBodyIndex :type Integer) (bFromSweep :type Boolean) (SweepResult :type "HitResult Structure (by ref)"))
  (if (not (`self.HasBeenCut?`))
    (bind _asbp_main_character (cast `/Game/Art/Character/MainCharacter/BP_MainCharacter` OtherActor))
    (bind _output_get (set `self.PlayerAttack` _asbp_main_character))
    (set `/Game/Gameplay/Training/Score.CutTitanNeck` true (`/Game/Art/Character/MainCharacter/BP_MainCharacter.Score` _output_get))
    (add `/Game/Art/Character/MainCharacter/BP_MainCharacter.AttackKey Released` (`self.PlayerAttack`) (delegate `AttackKey Released`))
    (goto _label_2 :!via `Open`)))

(event `self.Capsule.OnComponentEndOverlap`
  (params (OverlappedComponent :type "PrimitiveComponent Object Reference") (OtherActor :type "Actor Object Reference") (OtherComp :type "PrimitiveComponent Object Reference") (OtherBodyIndex :type Integer))
  (if (== OtherActor (`self.PlayerAttack`))
    (set `/Game/Gameplay/Training/Score.CutTitanNeck` false (`/Game/Art/Character/MainCharacter/BP_MainCharacter.Score` (`self.PlayerAttack`)))
    (goto _label_2 :!via `Close`)))

(event `Display Attack Slash`
  (bind (_returnvalue_location _returnvalue_rotation) (`KismetMathLibrary.BreakTransform` (`SceneComponent.K2_GetComponentToWorld` (`self.VelocityDirectionWhenNeckCut`))))
  (`|SpawnActorFromClass` "/Game/Gameplay/Effects/BP_AttackSlash.BP_AttackSlash_C" (`SceneComponent.K2_GetComponentToWorld` (`self.VelocityDirectionWhenNeckCut`)) "AlwaysSpawn" "OverrideRootScale")
  (`GameplayStatics.SpawnEmitterAtLocation` "/Game/Art/Effect/Particles/P_SmallSparks.P_SmallSparks" _returnvalue_location _returnvalue_rotation))

(fn `UserConstructionScript`)