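; World help icon that shows a help pop-up when the human player overlaps it, with title and color set in the construction script.
; Overlap creates UMG_Help_Frame at its switcher page, replacing any different page, and sets the controller's help menu index.
; The widget's timer stops on overlap and restarts on exit; a looping timer turns the title toward the camera.
; Spawn-point update needs TimeTrackerREF, whose lookup is unwired, as is icon spin.
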(event `self.Collision.OnComponentBeginOverlap`
  (params (OverlappedComponent :type "PrimitiveComponent Object Reference") (OtherActor :type "Actor Object Reference") (OtherComp :type "PrimitiveComponent Object Reference") (OtherBodyIndex :type Integer) (bFromSweep :type Boolean) (SweepResult :type "HitResult Structure (by ref)"))
  (bind _timetrackerref (`self.TimeTrackerREF`))
  (bind _umg_help_ref (`self.UMG Help REF`))
  (`/Engine/EditorBlueprintResources/StandardMacros.IsValid` _umg_help_ref
    (:`Is Valid`
      (`/Game/UI/HelpIcon/UMG_Help_Frame.Stop Timer` _umg_help_ref))
    (:`Is Not Valid`
      _))
  (bind _asbp_human_player_01 (cast `/Game/Gameplay/Characters/Player/BP_HumanPlayer_01` OtherActor))
  (bind _asbppc_human_player_01 (cast `/Game/Temp/NewCharacterMovement/PlayerController/BPPC_HumanPlayer_01` (`Pawn.GetController` _asbp_human_player_01)))
  (set `self.ControllerREF` _asbppc_human_player_01)
  (`|ExecutionSequence`
    (:`then_0`
      (bind _foundwidgets (`WidgetBlueprintLibrary.GetAllWidgetsOfClass` "/Game/UI/HelpIcon/UMG_Help_Frame.UMG_Help_Frame_C"))
      (bind _output (`|GetArrayItem` _foundwidgets))
      (`/Engine/EditorBlueprintResources/StandardMacros.IsValid` _output
        (:`Is Valid`
          (if (!= (`WidgetSwitcher.ActiveWidgetIndex` (`/Game/UI/HelpIcon/UMG_Help_Frame.WidgetSwitcher` _output)) (`self.WidgetSwitcher_Index`))
            (`Widget.RemoveFromParent` _output)
            (bind _returnvalue (`|CreateWidget` "/Game/UI/HelpIcon/UMG_Help_Frame.UMG_Help_Frame_C" (`self.ControllerREF`) :!label _label))
            (set `self.UMG Help REF` _returnvalue)
            (`WidgetSwitcher.SetActiveWidgetIndex` (`/Game/UI/HelpIcon/UMG_Help_Frame.WidgetSwitcher` _returnvalue) (`self.WidgetSwitcher_Index`))
            (`UserWidget.AddToViewport` _returnvalue 0)
            (if (`self.ActivateSpawnPoint?`)
              (`/Engine/EditorBlueprintResources/StandardMacros.IsValid` _timetrackerref
                (:`Is Valid`
                  (set `/Game/Gameplay/Training/BP_TimeTracker.CurrentPlayerStart` (`self.SpawnPoint`) _timetrackerref))))))
        (:`Is Not Valid`
          (goto _label))))
    (:`then_1`
      (set `/Game/Temp/NewCharacterMovement/PlayerController/BPPC_HumanPlayer_01.HelpMenu_Index` (`self.HelpMenu_Index`) (`self.ControllerREF`)))))

(event `self.ReceiveBeginPlay`
  (`KismetSystemLibrary.K2_SetTimer` null "Update Text Rotation" 0.01 true))

(event `self.ReceiveTick`
  (params (DeltaSeconds :type "Float (single-precision)")))

(event `self.Collision.OnComponentEndOverlap`
  (params (OverlappedComponent :type "PrimitiveComponent Object Reference") (OtherActor :type "Actor Object Reference") (OtherComp :type "PrimitiveComponent Object Reference") (OtherBodyIndex :type Integer))
  (bind _umg_help_ref (`self.UMG Help REF`))
  (`/Engine/EditorBlueprintResources/StandardMacros.IsValid` _umg_help_ref
    (:`Is Valid`
      (`/Game/UI/HelpIcon/UMG_Help_Frame.Set Timer` _umg_help_ref))))

(event `Update Text Rotation`
  ;[1 1 1] Face Text to Player
  (`SceneComponent.K2_SetWorldRotation` (`self.TextRender1`) (`KismetMathLibrary.MakeRotFromX` (- (`self.K2_GetActorLocation` (`GameplayStatics.GetPlayerCameraManager` 0)) (`SceneComponent.K2_GetComponentLocation` (`self.TextRender1`)))) false false))

(fn `UserConstructionScript`
  (`TextRenderComponent.K2_SetText` (`self.TextRender1`) (`self.Title`))
  (bind _returnvalue (`PrimitiveComponent.CreateDynamicMaterialInstance` (`self.HelpIcon`) 0 "/Game/Art/Environment/Training/MINST_BlueSimpleEmissive.MINST_BlueSimpleEmissive"))
  (`MaterialInstanceDynamic.SetVectorParameterValue` _returnvalue "EmissiveColor" (`self.ColorIcon`))
  (`TextRenderComponent.SetTextRenderColor` (`self.TextRender1`) (`KismetMathLibrary.Conv_LinearColorToColor` (`self.ColorIcon`))))