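; Hook projectile for the player's 3DMG gear that sticks to whatever it hits, including Titans.
; In flight, its collision sphere's radius scales with elapsed time, and a timeline changes gravity after a delay.
; On hit it stops, disables collision and attaches to the struck component's bone.
; A hooked BP_BigTitan_01 is notified on attach and again when DestroyHook releases it.
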(event `self.ReceiveHit`
  (params (MyComp :type "PrimitiveComponent Object Reference") (Other :type "Actor Object Reference") (OtherComp :type "PrimitiveComponent Object Reference") (bSelfMoved :type Boolean) (HitLocation :type "Vector Structure") (HitNormal :type "Vector Structure") (NormalImpulse :type "Vector Structure") (Hit :type "HitResult Structure (by ref)"))
  (bind (_bblockinghit _binitialoverlap _time _location _impactpoint _normal _impactnormal _physmat _hitactor _hitcomponent _hitbonename) (`GameplayStatics.BreakHitResult` Hit))
  (bind _projectilemovement (`self.ProjectileMovement`))
  ;[1 1 1] Stop Movement immediately when the projectile hit something, and attach the root to the actor that has been hit
  (set `self.Hit Something?` true)
  (`MovementComponent.StopMovementImmediately` _projectilemovement)
  (`ActorComponent.Deactivate` _projectilemovement)
  (`PrimitiveComponent.SetCollisionEnabled` (`self.Sphere`) "NoCollision")
  (`self.K2_AttachToComponent` _hitcomponent _hitbonename "KeepWorld" "KeepRelative" "KeepRelative")
  (bind _asbp_big_titan_01 (cast `/Game/Gameplay/Characters/Titans/BP_BigTitan_01` _hitactor))
  (bind _output_get (set `self.Titan hooked` _asbp_big_titan_01))
  (`/Game/Gameplay/Characters/Titans/BP_BigTitan_01.Has been hooked` _output_get (`self.Owner Player`))
  (set `self.Hit Titan?` true))

(event `self.ReceiveBeginPlay`
  (set `self.Initial Time ` (`GameplayStatics.GetTimeSeconds`))
  ;[1 1 1] Rise the gravity after a certain time
  (set `self.Initial Position` (`self.K2_GetActorLocation`))
  (`KismetSystemLibrary.Delay` (`self.DelayBeforeGravityRise`))
  (bind (_direction _gravity_scale) (`Timeline|Gravity Scale`)
    (:`Update`
      (set `ProjectileMovementComponent.ProjectileGravityScale` _gravity_scale (`self.ProjectileMovement`)))))

(event `Destroy Hook`
  ;[1 1 1] Destroy the Hook
  (`|ExecutionSequence`
    (:`then_0`
      (if (`self.Hit Titan?`)
        (`/Game/Gameplay/Characters/Titans/BP_BigTitan_01.Hook has been released` (`self.Titan hooked`) (`self.Owner Player`))))
    (:`then_1`
      (`self.K2_DestroyActor`))))

(event `self.ReceiveTick`
  (params (DeltaSeconds :type "Float (single-precision)"))
  (if (not (`self.Hit Something?`))
    (`SphereComponent.SetSphereRadius` (`self.Sphere`) (`KismetMathLibrary.MapRangeClamped` (- (`GameplayStatics.GetTimeSeconds`) (`self.Initial Time `)) 0.0 2.0 1.0 1000.0) true)))

(fn `Change Attack Type`
  (params (`Attack Type` :type "/Game/AI/Simple_Titan/ENUM_Big_Titan_Attacks Enum" :default "NewEnumerator2"))
  (returns (NewParam :type "/Game/AI/Simple_Titan/ENUM_Big_Titan_Attacks Enum"))
  (return "NewEnumerator2"))

(fn `UserConstructionScript`)