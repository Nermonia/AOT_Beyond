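; BP_SnapToGround is a level design Blueprint that places a configurable mesh on the surface above or below it.
; Its construction script adds a static mesh component and runs a vertical Visibility line trace, ProjectionSize long and centered on that component.
; On a hit, the component moves to the impact location without changing rotation, so snapping happens at construction rather than during gameplay.
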(fn `UserConstructionScript`
  (bind _returnvalue (/ (`self.ProjectionSize`) 2.0))
  (`AddComponent|StaticMeshComponent_442`)
  (bind _returnvalue_2 (`AddComponent|StaticMeshComponent_20`))
  (`StaticMeshComponent.SetStaticMesh` _returnvalue_2 (`self.Mesh`))
  (bind (_returnvalue_x _returnvalue_y _returnvalue_z) (`KismetMathLibrary.BreakVector` (`SceneComponent.K2_GetComponentLocation` _returnvalue_2)))
  (bind (_returnvalue_x_2 _returnvalue_y_2 _returnvalue_z_2) (`KismetMathLibrary.BreakVector` (`SceneComponent.K2_GetComponentLocation` _returnvalue_2)))
  (bind (_outhit _returnvalue_3) (`KismetSystemLibrary.LineTraceSingle` (`KismetMathLibrary.MakeVector` _returnvalue_x _returnvalue_y (+ _returnvalue_z _returnvalue)) (`KismetMathLibrary.MakeVector` _returnvalue_x_2 _returnvalue_y_2 (- _returnvalue_z_2 _returnvalue)) "TraceTypeQuery1"))
  (if _returnvalue_3
    (`SceneComponent.K2_SetWorldLocation` _returnvalue_2 (`.Location` (`GameplayStatics.BreakHitResult` _outhit)) false false)))