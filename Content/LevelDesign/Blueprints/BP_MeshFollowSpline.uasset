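; Level design tool that places copies of a static mesh at regular spacing along a spline, built entirely in the Construction Script.
; The spline length divided by Spacing sets the count, and one chosen index can be skipped to leave a gap.
; Each new component takes the spline's world location and yaw only, ignoring pitch and roll.
; Scale, position offsets and an axis-based orientation correction are then applied.
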(fn `UserConstructionScript`
  (locals (Local_Mesh :type "StaticMeshComponent Object Reference"))
  (bind _local_mesh (`local.Local_Mesh`))
  (bind _spline (`self.Spline`))
  (`|ExecutionSequence`
    (:`then_0`
      ;[1 1 1] Number of Indexes
      (set `self.LastIndex` (- (`.ReturnValue` (`KismetMathLibrary.FMod` (`SplineComponent.GetSplineLength`) (`self.Spacing`))) 1)))
    (:`then_1`
      (for _index (range (+ (`self.LastIndex`) 1))
        (if (not (== _index (`self.Mesh ID to hide`)))
          (bind _returnvalue (+ (* _index (`self.Spacing`)) (`self.MeshOffsetX`)))
          (bind _returnvalue_2 (`AddComponent|Static Mesh Component_9` :`bManualAttachment` true :`RelativeTransform` (`KismetMathLibrary.MakeTransform` (`SplineComponent.GetLocationAtDistanceAlongSpline` _spline _returnvalue "World") (`KismetMathLibrary.MakeRotator` 0.0 0.0 (.yaw (`SplineComponent.GetRotationAtDistanceAlongSpline` _spline _returnvalue "World"))) (1.0 1.0 1.0))))
          (set `local.Local_Mesh` _returnvalue_2)
          (`SceneComponent.SetWorldScale3D` (`local.Local_Mesh`) (`self.Scale`))
          (`StaticMeshComponent.SetStaticMesh` (`local.Local_Mesh`) (`self.Mesh`))
          (`SceneComponent.K2_AddLocalOffset` (`local.Local_Mesh`) (`KismetMathLibrary.MakeVector` 0.0 (`self.MeshOffsetY`) (`self.MeshOffsetZ`)) false false)
          (switch `/Game/LevelDesign/Blueprints/MeshFollowSpline_MeshOrientation` (`self.MeshOrientation`)
            (:`NewEnumerator1`
              (`SceneComponent.K2_AddLocalRotation` _local_mesh (struct :`Yaw` 90.0) false false))
            (:`NewEnumerator2`
              (`SceneComponent.K2_AddLocalRotation` _local_mesh (struct :`Pitch` 90.0) false false))
            (:`NewEnumerator3`
              (`SceneComponent.K2_AddLocalRotation` _local_mesh (struct :`Roll` 180.0) false false))
            (:`NewEnumerator4`
              (`SceneComponent.K2_AddLocalRotation` _local_mesh (struct :`Yaw` -90.0) false false))
            (:`NewEnumerator5`
              (`SceneComponent.K2_AddLocalRotation` _local_mesh (struct :`Pitch` -90.0) false false))))))))