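; BP_RoadTool is a level design tool that builds a road by repeating a mesh along a spline.
; Its construction script divides the spline length by Spacing and adds one spline mesh component per whole segment, leaving any remainder uncovered.
; Each segment takes world-space positions and Spacing-scaled direction tangents from the spline, using manual attachment and a configurable mesh and collision type.
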(fn `UserConstructionScript`
  (bind _spacing (`self.Spacing`))
  (bind _splinemesh (`self.SplineMesh`))
  (`|ExecutionSequence`
    (:`then_0`
      (set `self.LastIndex` (- (`.ReturnValue` (`KismetMathLibrary.FMod` (`SplineComponent.GetSplineLength`) (`self.Spacing`))) 1)))
    (:`then_1`
      (for _index (range (+ (`self.LastIndex`) 1))
        (bind _returnvalue (`AddComponent|Spline Mesh Component_0` :`bManualAttachment` true))
        (bind _output_get (set `self.SplineMesh` _returnvalue))
        (`StaticMeshComponent.SetStaticMesh` _output_get (`self.Mesh`))
        (`PrimitiveComponent.SetCollisionEnabled` _splinemesh (`self.CollisionType`))
        (bind _returnvalue_2 (* _index _spacing))
        (bind _returnvalue_3 (+ _returnvalue_2 _spacing))
        (`SplineMeshComponent.SetStartAndEnd` _splinemesh (`SplineComponent.GetWorldLocationAtDistanceAlongSpline` _returnvalue_2) (* (`SplineComponent.GetWorldDirectionAtDistanceAlongSpline` _returnvalue_2) _spacing) (`SplineComponent.GetWorldLocationAtDistanceAlongSpline` _returnvalue_3) (* (`SplineComponent.GetWorldDirectionAtDistanceAlongSpline` _returnvalue_3) _spacing) true)))))